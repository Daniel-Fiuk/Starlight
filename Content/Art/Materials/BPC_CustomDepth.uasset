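; Actor component that flashes its owner by setting custom depth stencil values, apparently as a damage hit effect.
; On BeginPlay it caches the owner's components of a configurable class.
; StartFlash has a damage-event signature, applies the Stencil value to those primitives and starts a short one-shot timer, while ResetStencil sets them back to zero.
; The binding to the owner's OnTakeAnyDamage is disconnected, so this component does not hook damage itself.
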(event Custom|StartFlash
  (params (DamagedActor :type Actor%20Object%20Reference) (Damage :type Float%20%28single-precision%29) (DamageType :type Damage%20Type%20Object%20Reference) (InstigatedBy :type Controller%20Object%20Reference) (DamageCauser :type Actor%20Object%20Reference))
  (for _array_element (Variables|Default|GetActorComponents)
    (bind _asprimitive_component (Utilities|Casting|CastToPrimitiveComponent _array_element))
    (Rendering|SetCustomDepthStencilValue _asprimitive_component (Variables|Default|GetStencil)))
  (bind _returnvalue (Utilities|Time|SetTimerbyEvent (EventDispatchers|CreateEvent :!event Custom|ResetStencil) 0.1))
  (Variables|Default|SetTimerHandle _returnvalue))

(event Custom|ResetStencil
  (for _array_element (Variables|Default|GetActorComponents)
    (bind _asprimitive_component (Utilities|Casting|CastToPrimitiveComponent _array_element))
    (Rendering|SetCustomDepthStencilValue _asprimitive_component 0)))

(event EventBeginPlay
  (Variables|Default|SetOwner (Components|GetOwner))
  (Variables|Default|SetActorComponents (Actor|GetComponentsByClass (Variables|Default|GetOwner) (Variables|Default|GetComponentClassToSearch))))