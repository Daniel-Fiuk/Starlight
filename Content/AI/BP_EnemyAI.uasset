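; Enemy AI Blueprint that detects the player and deals melee damage.
; Pawn sensing sets the "hasSeenPlayer?" blackboard key when it sees BP_MainCharacter.
; The MeleeAttack event runs a debug-drawn forward sphere trace, damages the player on a hit and sets the same key.
; The logic that clears the key is disconnected after the retriggerable delay, so the enemy never loses the player.
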(event OnSeePawn(PawnSensing)
  (params (Pawn :type Pawn%20Object%20Reference))
  ;[1 1 1] See Player
  (Utilities|Casting|CastToBP_MainCharacter Pawn)
  (AI|Components|Blackboard|SetValueasBool (AI|GetBlackboard (AI|GetAIController self)) (Utilities|Name|MakeLiteralName "hasSeenPlayer?") true)
  (Utilities|FlowControl|RetriggerableDelay 0.6))

(event Custom|MeleeAttack
  (bind _returnvalue (Transformation|GetActorLocation))
  ;[1 1 1] Melee Attack
  (bind (_outhit _returnvalue_2) (Collision|SphereTraceForObjects _returnvalue (+ _returnvalue (* (Math|Vector|GetForwardVector (Transformation|GetActorRotation)) 2.5e+02)) 8e+01 (Utilities|Array|MakeArray "ObjectTypeQuery3") false 0 "ForDuration"))
  (if _returnvalue_2
    (Utilities|Casting|CastToBP_MainCharacter (.HitActor (Collision|BreakHitResult _outhit)))
    (Development|PrintString "Attack")
    (Game|Damage|ApplyDamage (.HitActor (Collision|BreakHitResult _outhit)) 1e+01 0 0)
    (AI|Components|Blackboard|SetValueasBool (AI|GetBlackboard (AI|GetAIController self)) (Utilities|Name|MakeLiteralName "hasSeenPlayer?") true)
    (Utilities|FlowControl|RetriggerableDelay 0.6)))

(fn ConstructionScript)