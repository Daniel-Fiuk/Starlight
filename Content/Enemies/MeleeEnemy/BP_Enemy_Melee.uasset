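; Melee enemy character that fights with an equippable sword and can block incoming hits.
; Attack events pass montage and damage info to an attacks component for slash, jump, ground smash and spin attacks, with helpers for chasing, timeline mesh spinning and AOE damage limited to the attack target.
; Montage notifies spawn or destroy the socketed sword.
; Blockable damage randomly triggers a timed block before reaching the damage system component, which reports successful blocks for a react montage.
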(event OnBlocked(BPC_DamageSystem)
  (params (CanBeParried :type Boolean))
  ;[1 1 1] Blocking
  (Variables|Default|SetBlockingState "NewEnumerator2")
  (Utilities|Time|ClearandInvalidateTimerbyHandle (Variables|Default|GetHoldBlockTimer))
  (Animation|Montage|PlayMontage (Variables|Character|GetMesh) "/Game/Enemies/MeleeEnemy/Sword/Montages/Montage_Sword_React.Montage_Sword_React"
    (:OnCompleted
      _)
    (:OnInterrupted
      _))
  (CallFunction|EndBlock))

(event Custom|StartBlock
  ;[1 1 1] Blocking
  (Utilities|Time|ClearandInvalidateTimerbyHandle (Variables|Default|GetHoldBlockTimer))
  (Components|Movement|StopMovementImmediately (Variables|Character|GetCharacterMovement))
  (Variables|/Game/DamageSystem/BPC_DamageSystem.BPC_DamageSystem_C|SetIsBlocking (Variables|Default|GetBPC_DamageSystem) true)
  (Variables|Default|SetBlockingState "NewEnumerator1")
  (bind _returnvalue (Utilities|Time|SetTimerbyEvent (EventDispatchers|CreateEvent :!event Custom|EndBlock) 2.0))
  (Variables|Default|SetHoldBlockTimer _returnvalue))

(event Custom|EndBlock
  ;[1 1 1] Blocking
  (Variables|/Game/DamageSystem/BPC_DamageSystem.BPC_DamageSystem_C|SetIsBlocking (Variables|Default|GetBPC_DamageSystem) false)
  (Variables|Default|SetBlockingState "NewEnumerator0")
  (Default|CallOnBlockEnded))

(event Custom|StopSpinning
  ;[1 1 1] Attack Helpers
  (Audio|Components|Audio|Stop (Variables|Default|GetSpinMeshTimeline))
  (Transformation|SetRelativeRotation (Variables|Character|GetMesh) (Variables|Default|GetMeshRotationBeforeSpin) false false)
  (CallFunction|SetMovementSpeed "NewEnumerator3"))

(event Custom|AOESlash
  (params (AttackTarget :type Actor%20Object%20Reference))
  ;[1 1 1] Attack Helpers
  (bind _returnvalue (Game|SpawnActorfromClass "/Game/AttackSystem/AOE/BP_AOE_Base.BP_AOE_Base_C" (Math|Transform|MakeTransform (Transformation|GetActorLocation) "0, 0, 0" "1.000000,1.000000,1.000000") "Undefined" "MultiplyWithRoot" 0 false false false self))
  (Variables|/Game/AttackSystem/AOE/BP_AOE_Base.BP_AOE_Base_C|SetRadius _returnvalue 3e+02)
  (EventDispatchers|AssignOnAOEOverlapActor _returnvalue (delegate Custom|AOEDamageActor))
  (Default|Trigger _returnvalue))

(event Custom|AOEDamageActor
  (params (Actor :type Actor%20Object%20Reference))
  ;[1 1 1] Attack Helpers
  (if (== Actor (stale Custom|AOESlash AttackTarget))
    (Class|BPIDamagable|TakeDamage(Message) Actor (Utilities|Struct|MakeS_DamageInfo 1e+01 "NewEnumerator1" "NewEnumerator1") self)))

(event Custom|SpinMesh
  ;[1 1 1] Attack Helpers
  (Variables|Default|SetMeshRotationBeforeSpin (Variables|/Script/Engine.SceneComponent|GetRelativeRotation (Variables|Character|GetMesh)))
  (bind _zrotationalpha (Timeline|SpinMeshTimeline PlayFromStart)
    (:Update
      (Transformation|SetRelativeRotation (Variables|Character|GetMesh) (Math|Rotator|MakeRotator (.roll (Variables|Default|GetMeshRotationBeforeSpin)) (.pitch (Variables|Default|GetMeshRotationBeforeSpin)) (Math|Float|Lerp (.yaw (Variables|Default|GetMeshRotationBeforeSpin)) (+ (.yaw (Variables|Default|GetMeshRotationBeforeSpin)) 5.4e+03) _zrotationalpha)) false false))))

(event Custom|ShortRangeAttack
  (params (AttackTarget :type Actor%20Object%20Reference))
  ;[1 1 1] Attacks
  (Default|PrimaryMeleeAttack (Variables|Default|GetBPC_Attacks) (Utilities|Struct|MakeS_AttackInfo AttackTarget "/Game/Enemies/MeleeEnemy/Sword/Montages/Montage_SwordSlash.Montage_SwordSlash" (Utilities|Struct|MakeS_DamageInfo 1e+01 "NewEnumerator1")) 2e+01 2e+02))

(event Custom|SwordSpinAttack
  (params (AttackTarget :type Actor%20Object%20Reference))
  ;[1 1 1] Attacks
  (Default|SpinningAttack (Variables|Default|GetBPC_Attacks) (Utilities|Struct|MakeS_AttackInfo AttackTarget "/Game/Enemies/MeleeEnemy/Sword/Montages/Montage_Sword_SpinAttack.Montage_Sword_SpinAttack" (Utilities|Struct|MakeS_DamageInfo 1e+01 "NewEnumerator1"))))

(event Custom|LongRangeAttack
  (params (AttackTarget :type Actor%20Object%20Reference))
  ;[1 1 1] Attacks
  (Default|LongRangeMeleeAttack (Variables|Default|GetBPC_Attacks) (Utilities|Struct|MakeS_AttackInfo AttackTarget "/Game/Enemies/MeleeEnemy/Sword/Montages/Montage_Sword_JumpAttack.Montage_Sword_JumpAttack" (Utilities|Struct|MakeS_DamageInfo 2e+01 "NewEnumerator1")) 2e+01 2e+02))

(event Custom|GroundSmashAttack
  (params (AttackTarget :type Actor%20Object%20Reference))
  ;[1 1 1] Attacks
  (Default|GroundSmash (Variables|Default|GetBPC_Attacks) (Utilities|Struct|MakeS_AttackInfo AttackTarget "/Game/Enemies/MeleeEnemy/Sword/Montages/Montage_Melee_GroundSmash.Montage_Melee_GroundSmash" (Utilities|Struct|MakeS_DamageInfo 25.0 "NewEnumerator3")) 3e+02))

(event Custom|ChaseAttackTarget
  (params (AttackTarget :type Actor%20Object%20Reference))
  ;[1 1 1] Attack Helpers
  (CallFunction|SetMovementSpeed "NewEnumerator2")
  (AI|AIMoveTo self "0, 0, 0" AttackTarget 2e+02 false
    (:OnSuccess
      (Utilities|FlowControl|Delay 0.1)
      (if (Variables|Default|GetAttacking)
        (CallFunction|ChaseAttackTarget AttackTarget)))))

(event EventBeginPlay
  (|CallParentFunction))

(event EventUnequipWeapon
  ;[1 1 1] Equip Sword
  (bind _notifyname (Animation|Montage|PlayMontage (Variables|Character|GetMesh) "/Game/Enemies/MeleeEnemy/Sword/Montages/Montage_SheathSword.Montage_SheathSword")
    (:OnCompleted
      (Default|CallOnWeaponUnequipped))
    (:OnNotifyBegin
      (switch name _notifyname
        (:DropSword
          (Actor|DestroyActor (Variables|Default|GetWeaponActor))
          (Variables|Default|SetIsWieldingWeapon false))))))

(event EventEquipWeapon
  ;[1 1 1] Equip Sword
  (bind _notifyname (Animation|Montage|PlayMontage (Variables|Character|GetMesh) "/Game/Enemies/MeleeEnemy/Sword/Montages/Montage_UnsheathSword.Montage_UnsheathSword")
    (:OnCompleted
      (Default|CallOnWeaponEquipped))
    (:OnNotifyBegin
      (switch name _notifyname
        (:SpawnSword
          (bind _returnvalue (Game|SpawnActorfromClass "/Game/Weapons/BP_Weapon_Sword.BP_Weapon_Sword_C" (Transformation|GetActorTransform) "Undefined" "MultiplyWithRoot" 0 0))
          (bind _output_get (Variables|Default|SetWeaponActor _returnvalue))
          (Transformation|AttachComponentToComponent _output_get (Variables|Character|GetMesh) "hand_r_sword_socket" "SnapToTarget" "SnapToTarget" "SnapToTarget" true)
          (Variables|Default|SetIsWieldingWeapon true))))))

(fn ConstructionScript
  (|CallParentFunction)
  (Variables|Default|SetMeshRotationBeforeSpin (Variables|/Script/Engine.SceneComponent|GetRelativeRotation (Variables|Character|GetMesh))))

(fn TakeDamage
  (params (DamageInfo :type S%20Damage%20Info%20Structure) (Damage%20Causer :type Actor%20Object%20Reference))
  (if (Utilities|Struct|BreakS_DamageInfo DamageInfo)
    (CallFunction|TrytoBlock))
  (bind _wasdamaged (Default|TakeDamage (Variables|Default|GetBPC_DamageSystem) DamageInfo))
  (return _wasdamaged))

(fn TrytoBlock
  (if (<= (Math|Random|RandomFloat) (Variables|Default|GetBlockChance))
    (CallFunction|StartBlock)))

(fn CalculateFutureActorLocation
  (params (ActorTarget :type Actor%20Object%20Reference) (Time :type Float%20%28double-precision%29))
  (return (+ (Transformation|GetActorLocation ActorTarget) (* (* (Transformation|GetVelocity ActorTarget) "1.000000,1.000000,0.000000") Time))))

(fn GetIdealRange
  (return 2e+02 4e+02))