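; Adaptive music actor for the "Duel" track that layers drum, guitar and piano stems to match gameplay.
; BeginPlay starts five stems as UI sounds, then Tick reads boss state, player health, speed and combat to derive an Intensity level.
; UpdateVolumes sets stem multipliers: drums follow combat and speed, acoustic boss fights, strums combat and intensity, piano health, while lead guitar stays full.
; Delta-time steps fade most layers; sound-parameter code is left unwired.
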(event EventBeginPlay
  (bind _acousticright (Variables|Default|GetAcousticRight))
  (Class|AudioComponent|SetUISound _acousticright true)
  (Utilities|FlowControl|Sequence
    (:then_0
      (Audio|Components|Audio|Play _acousticright 0.0))
    (:then_1
      (Audio|Components|Audio|Play (Variables|Default|GetDrums) 0.0))
    (:then_2
      (Audio|Components|Audio|Play (Variables|Default|GetGutarStrum) 0.0))
    (:then_3
      (Audio|Components|Audio|Play (Variables|Default|GetPianoLeft) 0.0))
    (:then_4
      (Audio|Components|Audio|Play (Variables|Default|GetGuitarPrimary) 0.0))))

(event Collision|EventActorBeginOverlap
  (params (OtherActor :type Actor%20Object%20Reference)))

(event EventTick
  (params (DeltaSeconds :type Float%20%28single-precision%29))
  (bind _returnvalue (Game|GetGameInstance))
  (bind _bossfight (Class|BPIGlobalVariables|GetBossFight(Message) _returnvalue))
  (Variables|Default|SetInBossFight _bossfight)
  (bind _maxhealth (Class|BPIGlobalVariables|GetPlayerMaxHealth(Message) _returnvalue))
  (bind _health (Class|BPIGlobalVariables|GetPlayerHealth(Message) _returnvalue))
  (Variables|Default|SetHealth (/ _health _maxhealth))
  (bind _playerref (Class|BPIPlayer|GetPlayerRef(Message) (Game|GetPlayerCharacter 0)))
  (Variables|Default|SetSpeed (/ (Math|Vector|VectorLength (Variables|/Script/Engine.MovementComponent|GetVelocity (Pawn|GetMovementComponent _playerref))) (Class|MovementComponent|GetMaxSpeed (Pawn|GetMovementComponent _playerref))))
  (Variables|Default|SetInFight (> (Variables|/Game/Blueprints/Player/BP_Player.BP_Player_C|GetEnemiesInCombat _playerref) 0))
  (if (and (== (Math|Float|Round (Variables|Default|GetSpeed)) 1) (Variables|Default|GetInFight))
    (Variables|Default|SetIntensity 2)
    (elif (Variables|Default|GetInFight)
      (Variables|Default|SetIntensity 1)
      (elif (== (Math|Float|Round (Variables|Default|GetSpeed)) 1)
        (Variables|Default|SetIntensity 1)
        (else
          (Variables|Default|SetIntensity 0)))))
  (CallFunction|UpdateVolumes))

(fn ConstructionScript)

(fn UpdateVolumes
  (CallFunction|CalculateAmounts)
  (Audio|Components|Audio|SetVolumeMultiplier (Variables|Default|GetDrums) (Variables|Default|GetDrumsAmount) :!class /Script/Engine.AudioComponent)
  (Audio|Components|Audio|SetVolumeMultiplier (Variables|Default|GetAcousticRight) (Variables|Default|GetAcousticAmount) :!class /Script/Engine.AudioComponent)
  (Audio|Components|Audio|SetVolumeMultiplier (Variables|Default|GetAcousticLeft) (Variables|Default|GetAcousticAmount) :!class /Script/Engine.AudioComponent)
  (Audio|Components|Audio|SetVolumeMultiplier (Variables|Default|GetGutarStrum) (Variables|Default|GetGuitarStrumAmount) :!class /Script/Engine.AudioComponent)
  (Audio|Components|Audio|SetVolumeMultiplier (Variables|Default|GetGuitarStrumSlow) (Variables|Default|GetGuitarStrumSlowAmount) :!class /Script/Engine.AudioComponent)
  (Audio|Components|Audio|SetVolumeMultiplier (Variables|Default|GetPianoLeft) (Variables|Default|GetPianoAmount) :!class /Script/Engine.AudioComponent)
  (Audio|Components|Audio|SetVolumeMultiplier (Variables|Default|GetPianoRight) (Variables|Default|GetPianoAmount) :!class /Script/Engine.AudioComponent)
  (Audio|Components|Audio|SetVolumeMultiplier (Variables|Default|GetGuitarPrimary) (Variables|Default|GetGuitarPrimaryAmount) :!class /Script/Engine.AudioComponent))

(fn CalculateAmounts
  (Variables|Default|SetDrumsAmount (Math|Float|Clamp(Float) (* (Variables|Default|GetSpeed) (+ (select (Variables|Default|GetInFight) (Utilities|DeltaTimeTimes 2.0) (Utilities|DeltaTimeTimes -2.0)) (Variables|Default|GetDrumsAmount)))))
  (Variables|Default|SetAcousticAmount (Math|Float|Clamp(Float) (+ (select (Variables|Default|GetInBossFight) (Utilities|DeltaTimeTimes 2.0) (Utilities|DeltaTimeTimes -2.0)) (Variables|Default|GetAcousticAmount))))
  (Variables|Default|SetGuitarStrumAmount (Math|Float|Clamp(Float) (+ (+ (select (Variables|Default|GetInFight) (Utilities|DeltaTimeTimes 2.0) (Utilities|DeltaTimeTimes -2.0)) (select (> (Variables|Default|GetIntensity) 0) (Utilities|DeltaTimeTimes 2.0) (Utilities|DeltaTimeTimes -2.0))) (Variables|Default|GetGuitarStrumAmount))))
  (Variables|Default|SetGuitarStrumSlowAmount (Math|Float|Clamp(Float) (+ (+ (select (Variables|Default|GetInFight) (Utilities|DeltaTimeTimes 2.0) (Utilities|DeltaTimeTimes -2.0)) (select (> (Variables|Default|GetIntensity) 1) (Utilities|DeltaTimeTimes 2.0) (Utilities|DeltaTimeTimes -2.0))) (Variables|Default|GetGuitarStrumSlowAmount))))
  (Variables|Default|SetPianoAmount (Variables|Default|GetHealth))
  (Variables|Default|SetGuitarPrimaryAmount 1.0))