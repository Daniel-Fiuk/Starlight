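; Adaptive music Blueprint for Vi Prima Moenia that plays seven piano and instrument stems simultaneously, mixing them by player state.
; Each Tick sets stem volumes from four blend axes, then reads player state for the next update.
; Jumping favors piano, walking legato, menus the primary part, and greater height acoustic over electric.
; State-driven axes drift over time, their products weight each stem, and MultiplyCap boosts all but secondary legato electric.
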(event EventBeginPlay
  (bind _piano (Variables|Default|GetPiano))
  (Class|AudioComponent|SetUISound _piano true)
  (Audio|Components|Audio|Play _piano 0.0))

(event EventTick
  (params (DeltaSeconds :type Float%20%28single-precision%29))
  (CallFunction|UpdateVolume)
  (bind _playerref (Class|BPIPlayer|GetPlayerRef(Message) (Game|GetPlayerCharacter 0)))
  (Variables|Default|SetPlayer%20Ref _playerref)
  (Variables|Default|SetIsInMenu (Variables|/Game/Blueprints/Player/BP_Player.BP_Player_C|GetCurrentlyInMenu (Variables|Default|GetPlayer%20Ref)))
  (Variables|Default|SetIsWalking (Variables|/Game/Blueprints/Player/BP_Player.BP_Player_C|GetIsWalking (Variables|Default|GetPlayer%20Ref)))
  (Variables|Default|SetIsJumping (Variables|/Game/Blueprints/Player/BP_Player.BP_Player_C|GetIsJumping (Variables|Default|GetPlayer%20Ref)))
  (Variables|Default|SetPlayerHeight (Variables|/Game/Blueprints/Player/BP_Player.BP_Player_C|GetPlayersHeightInWorld (Variables|Default|GetPlayer%20Ref))))

(fn ConstructionScript)

(fn UpdateVolume
  ;[0.02732 0.001821 0.03955] Function: Update Volume
  ;;[1 1 1] Determine Audio Volume Scaling Amounts
  (CallFunction|CalculateAmounts)
  (CallFunction|CalculateAffectors)
  ;;;[0.0648 0.004777 0.09759] Update Volume
  (Variables|Default|SetMaxVol 1.5)
  (Audio|Components|Audio|SetVolumeMultiplier (Variables|Default|GetPiano) (Utilities|MultiplyCap (Variables|Default|GetPianoAmount) 4.0) :!class /Script/Engine.AudioComponent)
  (Audio|Components|Audio|SetVolumeMultiplier (Variables|Default|GetPrimaryLegatoAcoustic) (Utilities|MultiplyCap (Variables|Default|GetPrimaryLegatoAcousticAmount) 4.0) :!class /Script/Engine.AudioComponent)
  (Audio|Components|Audio|SetVolumeMultiplier (Variables|Default|GetPrimaryLegatoElectric) (Utilities|MultiplyCap (Variables|Default|GetPrimaryLegatoElectricAmount) 4.0) :!class /Script/Engine.AudioComponent)
  (Audio|Components|Audio|SetVolumeMultiplier (Variables|Default|GetPrimaryStaccatoAcoustic) (Utilities|MultiplyCap (Variables|Default|GetPrimaryStaccatoAcousticAmount) 4.0) :!class /Script/Engine.AudioComponent)
  (Audio|Components|Audio|SetVolumeMultiplier (Variables|Default|GetPrimaryStaccatoElectric) (Utilities|MultiplyCap (Variables|Default|GetPrimaryStaccatoElectricAmount) 4.0) :!class /Script/Engine.AudioComponent)
  (Audio|Components|Audio|SetVolumeMultiplier (Variables|Default|GetSecondaryLegatoAcoustic) (Utilities|MultiplyCap (Variables|Default|GetSecondaryLegatoAcousticAmount) 4.0) :!class /Script/Engine.AudioComponent)
  (Audio|Components|Audio|SetVolumeMultiplier (Variables|Default|GetSecondaryLegatoElectric) (Variables|Default|GetSecondaryLegatoElectricAmount) :!class /Script/Engine.AudioComponent))

(fn CalculateAmounts
  (bind _piano_guitar (Variables|Default|GetPiano/Guitar))
  (bind _acoustic_electric (Variables|Default|GetAcoustic/Electric))
  (bind _primary_secondary (Variables|Default|GetPrimary/Secondary))
  (bind _staccato_legato (Variables|Default|GetStaccato/Legato))
  (bind _returnvalue (- 1.0 _primary_secondary))
  (bind _returnvalue_2 (- 1.0 _staccato_legato))
  (bind _returnvalue_3 (- 1.0 _acoustic_electric))
  (bind _returnvalue_4 (* _piano_guitar _returnvalue))
  (bind _returnvalue_5 (* _piano_guitar _returnvalue_2))
  (bind _returnvalue_6 (* _piano_guitar _returnvalue_3))
  (bind _returnvalue_7 (- 1.0 _returnvalue_5))
  (bind _returnvalue_8 (- 1.0 _returnvalue_6))
  (bind _returnvalue_9 (- 1.0 _returnvalue_4))
  ;[0.06621 1 0.201] Values In
  ;[0 0.08333 0.00611] Values Out
  (Variables|Default|SetPianoAmount (- 1.0 _piano_guitar))
  ;;[0 1 0] PLA
  (Variables|Default|SetPrimaryLegatoAcousticAmount (* _returnvalue_4 _returnvalue_7 _returnvalue_6))
  ;;[0 1 1] PLE
  (Variables|Default|SetPrimaryLegatoElectricAmount (* _returnvalue_4 _returnvalue_7 _returnvalue_8))
  ;;[0 0 0] PSA
  (Variables|Default|SetPrimaryStaccatoAcousticAmount (* _returnvalue_4 _returnvalue_5 _returnvalue_6))
  ;;[0 0 1] PSE
  (Variables|Default|SetPrimaryStaccatoElectricAmount (* _returnvalue_4 _returnvalue_5 _returnvalue_8))
  ;;[1 1 0] SLA
  (Variables|Default|SetSecondaryLegatoAcousticAmount (* _returnvalue_9 _returnvalue_7 _returnvalue_6))
  ;;[1 1 1] SLE
  (Variables|Default|SetSecondaryLegatoElectricAmount (* _returnvalue_9 _returnvalue_7 _returnvalue_8))
  (return))

(fn CalculateAffectors
  (if (Variables|Default|GetIsJumping)
    ;[1 1 1] Increase Piano
    (Variables|Default|SetPiano/Guitar (Math|Float|Clamp(Float) (- (Variables|Default|GetPiano/Guitar) (* (Utilities|Time|GetWorldDeltaSeconds) (LocalVariables|GetadjustmentSpeed) 15.0)) 0.01 0.99))
    (else
      ;[1 1 1] Decrease Piano
      (Variables|Default|SetPiano/Guitar (Math|Float|Clamp(Float) (+ (Variables|Default|GetPiano/Guitar) (* (Utilities|Time|GetWorldDeltaSeconds) (LocalVariables|GetadjustmentSpeed) 1.0)) 0.01 0.8))))
  (if (Variables|Default|GetIsWalking)
    ;[1 1 1] Increase Legato
    (Variables|Default|SetStaccato/Legato (Math|Float|Clamp(Float) (+ (Variables|Default|GetStaccato/Legato) (* (Utilities|Time|GetWorldDeltaSeconds) (LocalVariables|GetadjustmentSpeed) 4.0)) 0.01 0.99))
    (else
      ;[1 1 1] Decrease Legato
      (Variables|Default|SetStaccato/Legato (Math|Float|Clamp(Float) (- (Variables|Default|GetStaccato/Legato) (* (Utilities|Time|GetWorldDeltaSeconds) (LocalVariables|GetadjustmentSpeed))) 0.01 0.99))))
  (if (Variables|Default|GetIsInMenu)
    ;[1 1 1] Decrease Secondary
    (Variables|Default|SetPrimary/Secondary (Math|Float|Clamp(Float) (- (Variables|Default|GetPrimary/Secondary) (* (Utilities|Time|GetWorldDeltaSeconds) (LocalVariables|GetadjustmentSpeed))) 0.01 0.99))
    (else
      ;[1 1 1] Increase Secondary
      (Variables|Default|SetPrimary/Secondary (Math|Float|Clamp(Float) (+ (Variables|Default|GetPrimary/Secondary) (* (Utilities|Time|GetWorldDeltaSeconds) (LocalVariables|GetadjustmentSpeed))) 0.01 0.8))))
  (Variables|Default|SetAcoustic/Electric (Math|Float|Clamp(Float) (* (- 1.0 (- (/ (Variables|Default|GetPlayerHeight) 1e+03) -0.1)) 2.0) 0.01 0.99)))