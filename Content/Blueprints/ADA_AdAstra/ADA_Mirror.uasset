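; Adaptive music actor that layers instrument stems according to level-generation progress.
; It starts six guitar, pad and piano tracks together as UI sounds, then each tick reads loading progress from WFC_Mk2_LevelGenerator.
; MediateAndClamp fades each stem in or out at a frame-rate-independent speed, based on its own progress threshold.
; UpdateVolumes zeroes the Piano volume after its fade step, so that stem stays muted.
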(event EventBeginPlay
  (bind _guitar_harmonics_left (Variables|Default|GetGuitar%20Harmonics%20Left))
  (Class|AudioComponent|SetUISound _guitar_harmonics_left true)
  (Audio|Components|Audio|Play _guitar_harmonics_left 0.0))

(event Collision|EventActorBeginOverlap
  (params (OtherActor :type Actor%20Object%20Reference)))

(event EventTick
  (params (DeltaSeconds :type Float%20%28single-precision%29))
  (bind _returnvalue (Actor|GetActorOfClass "/Game/Blueprints/WFC_Mk2_LevelGeneration/WFC_Mk2_LevelGenerator.WFC_Mk2_LevelGenerator_C"))
  (bind _percentage (Class|BPILevelGenerator|GetTilesSpawned(Message) _returnvalue))
  (Variables|Default|SetLoading%20Percentage _percentage)
  (CallFunction|UpdateVolumes))

(fn ConstructionScript)

(fn UpdateVolumes
  (bind _piano (Variables|Default|GetPiano))
  (Utilities|MediateandClamp (Variables|Default|GetGuitar%20Alternate) 0.7)
  (Utilities|MediateandClamp (Variables|Default|GetGuitar%20Harmonics%20Left) 0.1)
  (Utilities|MediateandClamp (Variables|Default|GetGuitar%20Harmonics%20Right) 0.2)
  (Utilities|MediateandClamp (Variables|Default|GetGuitar%20Primary) 0.0)
  (Utilities|MediateandClamp (Variables|Default|GetPads) 0.4)
  (Utilities|MediateandClamp _piano 0.6)
  (Audio|Components|Audio|SetVolumeMultiplier _piano 0.0 :!class /Script/Engine.AudioComponent))