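; Scuf_Spawnz_Comp is an actor component that gives its owner a random chance to spawn an extra actor when play begins.
; On BeginPlay it rolls a random integer against Rarity, so the spawn succeeds one time in Rarity.
; On success it spawns a random class from the Actors list at the owner's location plus Offset, ignoring collisions.
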(event EventBeginPlay
  (bind _rarity (Variables|Default|GetRarity))
  (if (== (- _rarity 1) (Math|Random|RandomInteger _rarity))
    (Game|SpawnActorfromClass (.OutItem (Utilities|Array|Random (Variables|Default|GetActors))) (Math|Conversions|ToTransform(Vector) (+ (Transformation|GetActorLocation (Components|GetOwner)) (Variables|Default|GetOffset))) "AlwaysSpawn" "MultiplyWithRoot" 0 0)))