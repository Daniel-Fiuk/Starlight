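; Enemy spawner that populates the level once, after its referenced Generator reports that generation is complete.
; Tick polls the completion flag and uses a Spawned boolean to fire only once.
; It then spawns EnemiesMax actors, each a random class from the Actors array, at random points in a fixed square around world origin at a constant height.
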(event EventBeginPlay)

(event Collision|EventActorBeginOverlap
  (params (OtherActor :type Actor%20Object%20Reference)))

(event EventTick
  (params (DeltaSeconds :type Float%20%28single-precision%29))
  (if (and (Variables|/Game/Blueprints/WFC_Mk2_LevelGeneration/WFC_Mk2_LevelGenerator.WFC_Mk2_LevelGenerator_C|GetGeneration%20Is%20Complete (Variables|Default|GetGenerator)) (not (Variables|Default|GetSpawned)))
    (Variables|Default|SetSpawned true)
    (for _index (range 1 (Variables|Default|GetEnemies%20Max))
      (Game|SpawnActorfromClass (.OutItem (Utilities|Array|Random (Variables|Default|GetActors))) (Math|Transform|MakeTransform (Math|Vector|MakeVector (Math|Random|RandomFloatinRange -3e+03 3e+03) (Math|Random|RandomFloatinRange -3e+03 3e+03) 1e+02)) "Undefined" "MultiplyWithRoot" 0 0))))

(fn ConstructionScript)