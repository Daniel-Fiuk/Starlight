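; BP_Interatable_Base is a base interactable actor that detects when the player is in range.
; Entering its SphereTrigger casts to BP_Player, caches that reference, shows the HUD interact prompt, enables actor input for player controller 0 and sets an Overlapping flag.
; Leaving the trigger hides the prompt, disables input and clears the flag.
; The file defines no interaction action itself.
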(event OnComponentBeginOverlap(SphereTrigger)
  (params (OverlappedComponent :type Primitive%20Component%20Object%20Reference) (OtherActor :type Actor%20Object%20Reference) (OtherComp :type Primitive%20Component%20Object%20Reference) (OtherBodyIndex :type Integer) (bFromSweep :type Boolean) (SweepResult :type Hit%20Result%20Structure%20%28by%20ref%29))
  (bind _asbp_player (Utilities|Casting|CastToBP_Player OtherActor))
  (Variables|Default|SetPlayerRef _asbp_player)
  (Default|ShowInteract (Variables|/Game/Blueprints/Player/BP_Player.BP_Player_C|GetPlayerHUDRef _asbp_player))
  (Input|EnableInput (Game|GetPlayerController 0))
  (Variables|Default|SetOverlapping true))

(event OnComponentEndOverlap(SphereTrigger)
  (params (OverlappedComponent :type Primitive%20Component%20Object%20Reference) (OtherActor :type Actor%20Object%20Reference) (OtherComp :type Primitive%20Component%20Object%20Reference) (OtherBodyIndex :type Integer))
  (bind _asbp_player (Utilities|Casting|CastToBP_Player OtherActor))
  (Default|HideIntertact (Variables|/Game/Blueprints/Player/BP_Player.BP_Player_C|GetPlayerHUDRef _asbp_player))
  (Input|DisableInput (Game|GetPlayerController 0))
  (Variables|Default|SetOverlapping false))

(fn ConstructionScript)