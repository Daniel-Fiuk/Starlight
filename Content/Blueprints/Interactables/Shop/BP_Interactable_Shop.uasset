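; Interactable shop where the player talks to a shopkeeper and then opens the shop.
; The first Interact press shows a random greeting from an intro, death or general DataTable, picked by GameInstance flags; the next hides it and opens the player's notebook.
; A closing event picks a goodbye table based on whether money was spent.
; Leaving the sphere trigger hides dialogue, resets shop state and clears those flags.
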(event OnComponentEndOverlap(SphereTrigger)
  (params (OverlappedComponent :type Primitive%20Component%20Object%20Reference) (OtherActor :type Actor%20Object%20Reference) (OtherComp :type Primitive%20Component%20Object%20Reference) (OtherBodyIndex :type Integer))
  (Utilities|Casting|CastToBP_Player OtherActor)
  (Class|BPIGlobalVariables|SetFirstRun(Message) (Game|GetGameInstance) false)
  (bind _dialogueui (Variables|Default|GetDialogueUI)
    (:then
      (Widget|SetVisibility _dialogueui "Hidden")
      (Variables|Default|SetStartedDialogue false)
      (Variables|Default|SetInShop false)
      (Variables|Default|SetSpentMoney false)
      (Class|BPIGlobalVariables|SetDied(Message) (Game|GetGameInstance) false))
    (:else)))

(event Custom|DisplayDialogueUI
  (bind _dialogueui (Variables|Default|GetDialogueUI)
    (:then
      (Widget|SetVisibility _dialogueui "Visible"))
    (:else
      (bind _returnvalue (UserInterface|CreateWidget "/Game/Widgets/UserInterface/HeadsUpDisplay/W_Dialogue.W_Dialogue_C" (Game|GetPlayerController 0) true))
      (bind _output_get (Variables|Default|SetDialogueUI _returnvalue))
      (UserInterface|Viewport|AddtoViewport _output_get 0))))

(event Custom|StartDialogue
  ;[1 1 1] Parts of Interaction
  (bind _firstrun (Class|BPIGlobalVariables|GetFirstRun(Message) (Game|GetGameInstance)))
  (if _firstrun
    (Variables|Default|SetDialogueType "/Game/Blueprints/Interactables/Shop/DT_IntroGreetings.DT_IntroGreetings")
    (else
      (bind _died (Class|BPIGlobalVariables|GetDied(Message) (Game|GetGameInstance)))
      (if _died
        (Variables|Default|SetDialogueType "/Game/Blueprints/Interactables/Shop/DT_DeathGreetings.DT_DeathGreetings")
        (else
          (Variables|Default|SetDialogueType "/Game/Blueprints/Interactables/Shop/DT_GeneralGreetings.DT_GeneralGreetings")))))
  (CallFunction|DisplayDialogue))

(event Custom|OpenShop
  ;[1 1 1] Parts of Interaction
  (if (not (Variables|Default|GetInShop))
    (bind _dialogueui (Variables|Default|GetDialogueUI)
      (:then
        (Widget|SetVisibility _dialogueui "Hidden")
        (bind _playerref (Class|BPIPlayer|GetPlayerRef(Message) (Game|GetPlayerCharacter 0)))
        (Default|OpenNotebook _playerref 3)
        (Variables|Default|SetInShop true))
      (:else))))

(event Custom|Closing%20Dialogue
  ;[1 1 1] Parts of Interaction
  (if (Variables|Default|GetSpentMoney)
    (Variables|Default|SetDialogueType "/Game/Blueprints/Interactables/Shop/DT_MoneyGoodbyes.DT_MoneyGoodbyes")
    (else
      (Variables|Default|SetDialogueType "/Game/Blueprints/Interactables/Shop/DT_CheapGoodbyes.DT_CheapGoodbyes")))
  (CallFunction|DisplayDialogue))

(event Custom|DisplayDialogue
  (bind _outrownames (DataTable|GetDataTableRowNames (Variables|Default|GetDialogueType)))
  (bind _returnvalue (Utilities|GetDataTableRow (Variables|Default|GetDialogueType) (Utilities|Array|Get(acopy) _outrownames (Math|Random|RandomIntegerinRange 0 (- (Utilities|Array|Length _outrownames) 1))))
    (:then
      (Class|BPIGlobalVariables|SetFirstRun(Message) (Game|GetGameInstance) false)
      (CallFunction|DisplayDialogueUI)
      (Rendering|Components|TextRender|SetText (Variables|/Game/Widgets/UserInterface/HeadsUpDisplay/W_Dialogue.W_Dialogue_C|GetDialogueText (Variables|Default|GetDialogueUI)) (Utilities|Struct|BreakS_Dialogue _returnvalue)))
    (:RowNotFound
      (Development|PrintString "Row Not Found"))))

(event Input|ActionEvents|InputActionInteract
  (params (Key :type Key%20Structure :default "None"))
  (:Pressed
    (if (Variables|Default|GetOverlapping)
      (Default|HideIntertact (Variables|/Game/Blueprints/Player/BP_Player.BP_Player_C|GetPlayerHUDRef (Variables|Default|GetPlayerRef)))
      (if (Variables|Default|GetStartedDialogue)
        (CallFunction|OpenShop)
        (else
          (CallFunction|StartDialogue)
          (Variables|Default|SetStartedDialogue true))))))

(fn ConstructionScript
  (|CallParentFunction))