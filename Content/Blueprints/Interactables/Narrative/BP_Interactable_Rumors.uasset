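; Interactable that shows the player a random rumor from the DT_Rumors data table in a dialogue widget when Interact is pressed while overlapping.
; It re-rolls rows until it finds one not in the Game Instance's heard-rumors list, clearing that list once every rumor has been heard.
; The dialogue widget is created once and reused, then hidden on leaving the trigger sphere, which also re-enables interaction.
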(event OnComponentEndOverlap(SphereTrigger)
  (params (OverlappedComponent :type Primitive%20Component%20Object%20Reference) (OtherActor :type Actor%20Object%20Reference) (OtherComp :type Primitive%20Component%20Object%20Reference) (OtherBodyIndex :type Integer))
  (Utilities|Casting|CastToBP_Player OtherActor)
  (bind _dialogueui (Variables|Default|GetDialogueUI)
    (:then
      (Widget|SetVisibility _dialogueui "Hidden")
      (Variables|Default|SetCanInteract true))
    (:else)))

(event Custom|DisplayDialogueUI
  (bind _dialogueui (Variables|Default|GetDialogueUI)
    (:then
      (Widget|SetVisibility _dialogueui "Visible"))
    (:else
      (bind _returnvalue (UserInterface|CreateWidget "/Game/Widgets/UserInterface/HeadsUpDisplay/W_Dialogue.W_Dialogue_C" (Game|GetPlayerController 0)))
      (bind _output_get (Variables|Default|SetDialogueUI _returnvalue))
      (UserInterface|Viewport|AddtoViewport _output_get 0))))

(event Input|ActionEvents|InputActionInteract
  (params (Key :type Key%20Structure :default "None"))
  (:Pressed
    (if (and (Variables|Default|GetOverlapping) (Variables|Default|GetCanInteract))
      (Default|HideIntertact (Variables|/Game/Blueprints/Player/BP_Player.BP_Player_C|GetPlayerHUDRef (Variables|Default|GetPlayerRef)))
      (bind _outrownames (DataTable|GetDataTableRowNames "/Game/Blueprints/Interactables/Narrative/DT_Rumors.DT_Rumors" :!label _label))
      (bind _returnvalue (Utilities|GetDataTableRow "/Game/Blueprints/Interactables/Narrative/DT_Rumors.DT_Rumors" (Utilities|Array|Get(acopy) _outrownames (Math|Random|RandomIntegerinRange 0 (- (Utilities|Array|Length _outrownames) 1))))
        (:then
          (bind _heardrumors (Class|BPIGlobalVariables|GetHeardRumors(Message) (Game|GetGameInstance)))
          (if (Utilities|Array|ContainsItem _heardrumors (Utilities|Struct|BreakS_Dialogue _returnvalue))
            (bind _outrownames_2 (DataTable|GetDataTableRowNames "/Game/Blueprints/Interactables/Narrative/DT_Rumors.DT_Rumors"))
            (if (== (Utilities|Array|Length _outrownames_2) (Utilities|Array|Length _heardrumors))
              (Class|BPIGlobalVariables|ResetHeardRumors(Message) (Game|GetGameInstance))
              (goto _label)
              (else
                (goto _label)))
            (else
              (Class|BPIGlobalVariables|AddHeardRumor(Message) (Game|GetGameInstance) (Utilities|Struct|BreakS_Dialogue _returnvalue))
              (CallFunction|DisplayDialogueUI)
              (Rendering|Components|TextRender|SetText (Variables|/Game/Widgets/UserInterface/HeadsUpDisplay/W_Dialogue.W_Dialogue_C|GetDialogueText (Variables|Default|GetDialogueUI)) (Utilities|Struct|BreakS_Dialogue _returnvalue))
              (Variables|Default|SetCanInteract false))))
        (:RowNotFound
          (Development|PrintString "Row Not Found"))))))

(fn ConstructionScript
  (|CallParentFunction))