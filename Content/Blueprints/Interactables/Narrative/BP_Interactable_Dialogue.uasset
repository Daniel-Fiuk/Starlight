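; Narrative interactable that steps through an array of dialogue lines each time Interact is pressed while Overlapping is true.
; Each press hides the HUD prompt, increments TalkIndex, then shows that line in a lazily created, reused W_Dialogue widget, hiding it once lines run out.
; Leaving SphereTrigger resets TalkIndex to 0 without hiding the widget; because increment precedes display, the next conversation starts at element 1.
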(event OnComponentEndOverlap(SphereTrigger)
  (params (OverlappedComponent :type Primitive%20Component%20Object%20Reference) (OtherActor :type Actor%20Object%20Reference) (OtherComp :type Primitive%20Component%20Object%20Reference) (OtherBodyIndex :type Integer))
  (Variables|Default|SetTalkIndex 0))

(event Custom|DisplayDialogueUI
  (bind _dialogueui (Variables|Default|GetDialogueUI)
    (:then
      (Widget|SetVisibility _dialogueui "Visible"))
    (:else
      (bind _returnvalue (UserInterface|CreateWidget "/Game/Widgets/UserInterface/HeadsUpDisplay/W_Dialogue.W_Dialogue_C" (Game|GetPlayerController 0)))
      (bind _output_get (Variables|Default|SetDialogueUI _returnvalue))
      (UserInterface|Viewport|AddtoViewport _output_get 0))))

(event Input|ActionEvents|InputActionInteract
  (params (Key :type Key%20Structure :default "None"))
  (:Pressed
    (if (Variables|Default|GetOverlapping)
      (Default|HideIntertact (Variables|/Game/Blueprints/Player/BP_Player.BP_Player_C|GetPlayerHUDRef (Variables|Default|GetPlayerRef)))
      (Math|Integer|IncrementInt (Variables|Default|GetTalkIndex)
        (:%20%20
          (if (< (Variables|Default|GetTalkIndex) (Utilities|Array|Length (Variables|Default|GetDialogue)))
            (CallFunction|DisplayDialogueUI)
            (Rendering|Components|TextRender|SetText (Variables|/Game/Widgets/UserInterface/HeadsUpDisplay/W_Dialogue.W_Dialogue_C|GetDialogueText (Variables|Default|GetDialogueUI)) (Utilities|Text|ToText(String) (Utilities|Array|Get(acopy) (Variables|Default|GetDialogue) (Variables|Default|GetTalkIndex))))
            (else
              (Widget|SetVisibility (Variables|Default|GetDialogueUI) "Hidden"))))))))

(fn ConstructionScript
  (|CallParentFunction))