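; Interactable teleporter that currently only prints "Teleport" instead of moving the player.
; On BeginPlay it spawns a large sparks emitter at its location.
; Pressing Interact while overlapping hides the HUD interact prompt through PlayerRef and prints the debug string.
; A node to open level Demo1 exists but is not connected, so it never runs.
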(event EventBeginPlay
  (Effects|SpawnEmitteratLocation "/Game/StarterContent/Particles/P_Sparks.P_Sparks" (Transformation|GetActorLocation) "0, 0, 0" "10.000000,10.000000,10.000000"))

(event Input|ActionEvents|InputActionInteract
  (params (Key :type Key%20Structure :default "None"))
  (:Pressed
    (if (Variables|Default|GetOverlapping)
      (Default|HideIntertact (Variables|/Game/Blueprints/Player/BP_Player.BP_Player_C|GetPlayerHUDRef (Variables|Default|GetPlayerRef)))
      (Development|PrintString "Teleport"))))

(fn ConstructionScript
  (|CallParentFunction))