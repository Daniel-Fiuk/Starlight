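; Interactable pickup that grants the player a random spell from the DT_Spells data table.
; On BeginPlay it picks a random row from the table and stores it as its Spell.
; Pressing Interact while overlapping adds the spell to the player's inventory component, shows a HUD notification with its icon and name, then destroys the actor.
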(event EventBeginPlay
  (bind _outrownames (DataTable|GetDataTableRowNames "/Game/Blueprints/MSC_MagicSystem/SpellInfo/DT_Spells.DT_Spells"))
  (bind _returnvalue (Utilities|GetDataTableRow "/Game/Blueprints/MSC_MagicSystem/SpellInfo/DT_Spells.DT_Spells" (Utilities|Array|Get(acopy) _outrownames (Math|Random|RandomIntegerinRange 0 (- (Utilities|Array|Length _outrownames) 1))))
    (:then
      (Variables|Default|SetSpell _returnvalue))))

(event Input|ActionEvents|InputActionInteract
  (params (Key :type Key%20Structure :default "None"))
  (bind _playerref (Variables|Default|GetPlayerRef))
  (bind _spell (Variables|Default|GetSpell))
  (bind (_icon _name) (Utilities|Struct|BreakS_SpellInfo _spell))
  (:Pressed
    (if (Variables|Default|GetOverlapping)
      (Default|AddItem (Variables|/Game/Blueprints/Player/BP_Player.BP_Player_C|GetBPC_Inventory _playerref) (Variables|Default|GetSpell))
      (Default|ShowNotification (Variables|/Game/Blueprints/Player/BP_Player.BP_Player_C|GetPlayerHUDRef _playerref) _icon _name)
      (Actor|DestroyActor))))

(fn ConstructionScript
  (|CallParentFunction))