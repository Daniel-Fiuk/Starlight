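; Interactable health potion pickup that the player collects by pressing Interact while overlapping it.
; On pickup it calls SetHealthPotionsMessage on the game instance with a value of one, then refreshes the player's potion UI.
; It shows a HUD notification with the potion icon and name, then destroys itself.
; The construction script only calls its parent's.
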(event Input|ActionEvents|InputActionInteract
  (params (Key :type Key%20Structure :default "None"))
  (bind _playerref (Variables|Default|GetPlayerRef))
  (:Pressed
    (if (Variables|Default|GetOverlapping)
      (Class|BPIGlobalVariables|SetHealthPotions(Message) (Game|GetGameInstance) 1)
      (Default|UpdatePotionUI _playerref)
      (Default|ShowNotification (Variables|/Game/Blueprints/Player/BP_Player.BP_Player_C|GetPlayerHUDRef _playerref) "/Game/Art/User_Interface/Notebook/PotionIcon.PotionIcon" "Health Potion")
      (Actor|DestroyActor))))

(fn ConstructionScript
  (|CallParentFunction))