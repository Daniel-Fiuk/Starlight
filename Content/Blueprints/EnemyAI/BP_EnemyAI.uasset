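; Enemy AI Blueprint that detects the player and deals melee or ranged damage to it.
; PawnSensing sets a "has seen player" Blackboard flag when it spots BP_MainCharacter.
; AttackPlayer picks melee or ranged from flags, both using forward sphere traces with debug drawing; ranged reaches farther for less damage, without projectiles.
; Tick rotates the health bar widget toward the player camera.
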(event OnSeePawn(PawnSensing)
  (params (Pawn :type Pawn%20Object%20Reference))
  ;[1 1 1] See Player
  (Utilities|Casting|CastToBP_MainCharacter Pawn)
  (AI|Components|Blackboard|SetValueasBool (AI|GetBlackboard (AI|GetAIController self)) (Utilities|Name|MakeLiteralName "hasSeenPlayer?") true))

(event Custom|MeleeAttack
  (bind _returnvalue (Transformation|GetActorLocation))
  ;[1 1 1] Melee Attack
  (if (Variables|Default|GetisMelee?)
    (bind (_outhit _returnvalue_2) (Collision|SphereTraceForObjects _returnvalue (+ _returnvalue (* (Math|Vector|GetForwardVector (Transformation|GetActorRotation)) 1.5e+02)) 8e+01 (Utilities|Array|MakeArray "ObjectTypeQuery3") false 0 "ForDuration"))
    (if _returnvalue_2
      (Utilities|Casting|CastToBP_MainCharacter (.HitActor (Collision|BreakHitResult _outhit)))
      (Game|Damage|ApplyDamage (.HitActor (Collision|BreakHitResult _outhit)) 15.0 0 0))))

(event Custom|RangeAttack
  (bind _returnvalue (Transformation|GetActorLocation))
  ;[1 1 1] Range Attack
  (if (Variables|Default|GetisRanged?)
    (bind (_outhit _returnvalue_2) (Collision|SphereTraceForObjects _returnvalue (+ _returnvalue (* (Math|Vector|GetForwardVector (Transformation|GetActorRotation)) 4.5e+02)) 8e+01 (Utilities|Array|MakeArray "ObjectTypeQuery3") false 0 "ForDuration"))
    (if _returnvalue_2
      (Utilities|Casting|CastToBP_MainCharacter (.HitActor (Collision|BreakHitResult _outhit)))
      (Game|Damage|ApplyDamage (.HitActor (Collision|BreakHitResult _outhit)) 1e+01 0 0))))

(event Custom|AttackPlayer
  ;[1 1 1] Start Attacks
  (if (Variables|Default|GetisMelee?)
    (CallFunction|MeleeAttack)
    (elif (Variables|Default|GetisRanged?)
      (CallFunction|RangeAttack))))

(event EventTick
  (params (DeltaSeconds :type Float%20%28single-precision%29))
  (bind _healthbarwidget (Variables|Default|GetHealthBarWidget))
  (Transformation|SetWorldRotation _healthbarwidget (Math|Rotator|FindLookatRotation (Transformation|GetWorldLocation _healthbarwidget) (Transformation|GetWorldLocation (Variables|/Script/Engine.PlayerCameraManager|GetTransformComponent (Game|GetPlayerCameraManager 0)))) false false))

(fn ConstructionScript)