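; Enemy AI child Blueprint configured by enum presets for speed, detection range, attack type and health.
; BeginPlay maps those presets to walk speed, PawnSensing sight radius, melee/ranged flags and starting health.
; Tick pushes the health ratio to the W_EnemyHealthBar widget every frame.
; AnyDamage subtracts health and destroys the actor only when health equals exactly zero, so overkill damage leaves it alive.
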(event EventTick
  (params (DeltaSeconds :type Float%20%28single-precision%29))
  (bind _asw_enemy_health_bar (Utilities|Casting|CastToW_EnemyHealthBar (UserInterface|GetWidget (Variables|Default|GetHealthBarWidget))))
  (Progress|SetPercent (Variables|/Game/UserInterface/HeadsUpDisplay/W_EnemyHealthBar.W_EnemyHealthBar_C|GetHealthBar _asw_enemy_health_bar) (/ (Variables|Default|GetcurrentHealth) (Variables|Default|GetmaxHealth))))

(event Game|Damage|EventAnyDamage
  (params (Damage :type Float%20%28single-precision%29) (DamageType :type Damage%20Type%20Object%20Reference) (InstigatedBy :type Controller%20Object%20Reference) (DamageCauser :type Actor%20Object%20Reference))
  (Variables|Default|SetcurrentHealth (- (Variables|Default|GetcurrentHealth) Damage))
  (if (== (Variables|Default|GetcurrentHealth) 0.0)
    (Actor|DestroyActor)))

(event EventBeginPlay
  (bind _pawnsensing (Variables|Default|GetPawnSensing))
  (bind _charactermovement (Variables|Character|GetCharacterMovement))
  ;[1 1 1] Enemy Speed
  (switch Utilities|FlowControl|Switch|SwitchonEnemySpeed (Variables|Default|GetEnemySpeed)
    (:NewEnumerator0
      (Variables|/Script/Engine.CharacterMovementComponent|SetMaxWalkSpeed _charactermovement 2e+02))
    (:NewEnumerator1
      (Variables|/Script/Engine.CharacterMovementComponent|SetMaxWalkSpeed _charactermovement 4e+02))
    (:NewEnumerator2
      (Variables|/Script/Engine.CharacterMovementComponent|SetMaxWalkSpeed _charactermovement 6e+02)))
  ;[1 1 1] Detection Range
  (switch Utilities|FlowControl|Switch|SwitchonEnemyDetectionRange (Variables|Default|GetEnemyDetectionRange)
    (:NewEnumerator0
      (Variables|/Script/AIModule.PawnSensingComponent|SetSightRadius _pawnsensing 1.5e+03))
    (:NewEnumerator1
      (Variables|/Script/AIModule.PawnSensingComponent|SetSightRadius _pawnsensing 4e+03))
    (:NewEnumerator2
      (Variables|/Script/AIModule.PawnSensingComponent|SetSightRadius _pawnsensing 6e+03)))
  ;[1 1 1] Attack Type
  (switch Utilities|FlowControl|Switch|SwitchonEnemyAttackType (Variables|Default|GetEnemyAttackType)
    (:NewEnumerator0
      (Variables|Default|SetisMelee? true)
      (Variables|Default|SetisRanged? false))
    (:NewEnumerator1
      (Variables|Default|SetisMelee? false)
      (Variables|Default|SetisRanged? true)))
  ;[1 1 1] Health
  (switch Utilities|FlowControl|Switch|SwitchonEnemyHealth (Variables|Default|GetEnemyHealth)
    (:NewEnumerator0
      (Variables|Default|SetmaxHealth 6e+01)
      (Variables|Default|SetcurrentHealth 6e+01))
    (:NewEnumerator1
      (Variables|Default|SetmaxHealth 1e+02)
      (Variables|Default|SetcurrentHealth 1e+02))
    (:NewEnumerator2
      (Variables|Default|SetmaxHealth 2e+02)
      (Variables|Default|SetcurrentHealth 2e+02))))

(fn ConstructionScript
  (|CallParentFunction))