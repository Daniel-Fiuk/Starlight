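; BP_NotePickup is a collectible note that unlocks a journal page when the player picks it up.
; Overlapping its ItemTrigger with BP_MainCharacter enables input, sets IsNear and shows the hotbar's interact prompt; leaving reverses this.
; Pressing E while near increments PagesUnlocked on the character's journal, using the actor from the overlap event, then destroys the pickup without explicitly hiding the prompt.
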(event OnComponentBeginOverlap(ItemTrigger)
  (params (OverlappedComponent :type Primitive%20Component%20Object%20Reference) (OtherActor :type Actor%20Object%20Reference) (OtherComp :type Primitive%20Component%20Object%20Reference) (OtherBodyIndex :type Integer) (bFromSweep :type Boolean) (SweepResult :type Hit%20Result%20Structure%20%28by%20ref%29))
  (bind _asbp_main_character (Utilities|Casting|CastToBP_MainCharacter OtherActor))
  (Input|EnableInput (Game|GetPlayerController 0))
  (Default|ShowInteract (Variables|/Game/Blueprints/Player/BP_MainCharacter.BP_MainCharacter_C|GetHotbarWidgetRef _asbp_main_character))
  (Variables|Default|SetisNear? true))

(event OnComponentEndOverlap(ItemTrigger)
  (params (OverlappedComponent :type Primitive%20Component%20Object%20Reference) (OtherActor :type Actor%20Object%20Reference) (OtherComp :type Primitive%20Component%20Object%20Reference) (OtherBodyIndex :type Integer))
  (bind _asbp_main_character (Utilities|Casting|CastToBP_MainCharacter OtherActor))
  (Input|DisableInput (Game|GetPlayerController 0) 0)
  (Default|HideInteract (Variables|/Game/Blueprints/Player/BP_MainCharacter.BP_MainCharacter_C|GetHotbarWidgetRef _asbp_main_character))
  (Variables|Default|SetisNear? false))

(event Input|KeyboardEvents|E
  (params (Key :type Key%20Structure :default "None"))
  (:Pressed
    (bind _asbp_main_character (Utilities|Casting|CastToBP_MainCharacter (stale OnComponentBeginOverlap(ItemTrigger) OtherActor)))
    (if (Variables|Default|GetisNear?)
      (Variables|/Game/UserInterface/HeadsUpDisplay/W_Journal.W_Journal_C|SetPagesUnlocked (Variables|/Game/Blueprints/Player/BP_MainCharacter.BP_MainCharacter_C|GetJournalRef _asbp_main_character) (+ (Variables|/Game/UserInterface/HeadsUpDisplay/W_Journal.W_Journal_C|GetPagesUnlocked (Variables|/Game/Blueprints/Player/BP_MainCharacter.BP_MainCharacter_C|GetJournalRef _asbp_main_character)) 1))
      (Actor|DestroyActor))))

(fn ConstructionScript)