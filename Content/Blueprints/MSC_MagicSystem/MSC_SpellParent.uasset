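; MSC_SpellParent is the base spell class for the magic system, defining cast, tick and hit behavior functions.
; The base cast stores the target position, spawns an MSC_SpellPrefab at the spell manager's owner, applies the projectile particle, and returns the projectile and cooldown.
; Each projectile keeps a reference to the MSC_SpellManagerComponent that spawned it.
; Tick and hit behaviors are empty stubs.
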(event EventBeginPlay)

(event EventTick
  (params (DeltaSeconds :type Float%20%28single-precision%29)))

(fn SpellonCastBehaviorBase
  (params (Self%20In :type Actor%20Component%20Object%20Reference) (Target%20Pos :type Vector))
  (Variables|Default|SetTarget%20Pos Target%20Pos)
  (bind _returnvalue (|SpawnProjectileActor Self%20In))
  (|SetParticle _returnvalue)
  (return (Utilities|Array|MakeArray _returnvalue) (Variables|Default|GetBase%20Cooldown)))

(fn SpellEventTickBehaviorBase
  (params (Spell%20Objs%20In :type Array%20of%20Object%20Object%20References))
  (return))

(fn SpellHit
  (params (Active%20Spells%20In :type Array%20of%20MSC%20Spell%20Prefab%20Object%20References) (Spell%20Obj%20In :type MSC%20Spell%20Prefab%20Object%20Reference))
  (return))