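; Base projectile actor for a spell in the MSC magic system, with a limited number of bounces.
; Sphere hits are reported to the spell manager component, flagged for destruction once no bounces remain.
; Each projectile bounce decrements the counter, with a short cooldown against double counting and a debug print.
; DestroySpell disables bouncing and destroys the actor after a delay only when bounces are spent, while ClearSpell does delayed destruction unconditionally.
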(event OnProjectileBounce(ProjectileMovement)
  (params (ImpactResult :type Hit%20Result%20Structure%20%28by%20ref%29) (ImpactVelocity :type Vector%20%28by%20ref%29 :default "0, 0, 0"))
  (if (not (Variables|Default|GetBounce%20On%20Cooldown))
    (Variables|Default|SetBounce%20On%20Cooldown true)
    (bind _result (Math|Integer|DecrementInt (Variables|Default|GetBounces))
      (:%20%20
        (Development|PrintString (Utilities|String|ToString(Integer) _result))
        (Utilities|FlowControl|Delay 0.2)
        (Variables|Default|SetBounce%20On%20Cooldown false)))))

(event OnComponentHit(Sphere)
  (params (HitComponent :type Primitive%20Component%20Object%20Reference) (OtherActor :type Actor%20Object%20Reference) (OtherComp :type Primitive%20Component%20Object%20Reference) (NormalImpulse :type Vector :default "0, 0, 0") (Hit :type Hit%20Result%20Structure%20%28by%20ref%29))
  (Default|MSCSpellHit (Variables|Default|GetMSC_SpellManagerComponent) self HitComponent OtherActor OtherComp NormalImpulse Hit (<= (Variables|Default|GetBounces) 0)))

(event Custom|Clear%20Spell
  (params (Delay :type Float%20%28single-precision%29))
  (Utilities|FlowControl|Delay Delay)
  (Actor|DestroyActor))

(event Custom|Destroy%20Spell
  (params (Delay :type Float%20%28single-precision%29))
  (bind _projectilemovement (Variables|Default|GetProjectileMovement))
  (if (<= (Variables|Default|GetBounces) 0)
    (Variables|/Script/Engine.ProjectileMovementComponent|SetbShouldBounce _projectilemovement false)
    (Variables|/Script/Engine.ProjectileMovementComponent|SetBounciness _projectilemovement 0.0)
    (Utilities|FlowControl|Delay Delay)
    (Actor|DestroyActor)))

(event EventBeginPlay)

(fn ConstructionScript)