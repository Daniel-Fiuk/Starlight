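; Spell manager component for the MagicSystem that builds, casts and updates a modular spell made of one base spell and a list of modifiers.
; Regenerating checks class types, destroys old components and adds the spell and mods to the owner as components.
; Casts are cooldown-gated: the base spawns spells and sets the cooldown, then each mod adjusts it.
; Active spells are ticked through base and mods, while hits go only to the base.
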(event Custom|MSC%20Cast%20Spell
  (params (Target%20Pos :type Vector) (Self%20In :type Actor%20Object%20Reference))
  (bind _self self)
  (bind _spell_data (Variables|Default|GetSpell%20Data))
  (if (<= (Variables|Default|GetCurrent%20Cooldown) 0.0)
    (bind _asmsc_spell_parent (Utilities|Casting|CastToMSC_SpellParent (.parent _spell_data)))
    (bind (_cast_spells_out _base_cooldown) (Default|SpellonCastBehaviorBase _asmsc_spell_parent _self Target%20Pos))
    (bind _output_get (Variables|Default|SetSpells%20Casted _cast_spells_out))
    (bind _output_get_2 (Variables|Default|SetCurrent%20Cooldown _base_cooldown))
    (for _array_element (.mods _spell_data)
      (bind _asmsc_spell_mod_parent (Utilities|Casting|CastToMSC_SpellModParent _array_element))
      (bind _cooldown_out (Default|SpellonCastBehaviorModification _asmsc_spell_mod_parent _output_get _asmsc_spell_parent _self Target%20Pos _output_get_2))
      (Variables|Default|SetCurrent%20Cooldown _cooldown_out))
    (Utilities|Array|AppendArray (Variables|Default|GetCurrent%20Active%20Spells) _output_get)))

(event Custom|MSC%20Regenerate%20Spell
  (params (Spell%20In :type Actor%20Component%20Class%20Reference) (Mods%20In :type Array%20of%20Actor%20Component%20Class%20References))
  (CallFunction|GenerateSpell Spell%20In Mods%20In))

(event Custom|MSC%20Spell%20Hit
  (params (Spell :type Actor%20Object%20Reference) (Hit%20Component :type Primitive%20Component%20Object%20Reference) (Other%20Actor :type Actor%20Object%20Reference) (Other%20Comp :type Primitive%20Component%20Object%20Reference) (Normal%20Vector :type Vector) (Hit :type Hit%20Result%20Structure))
  (bind _asmsc_spell_parent (Utilities|Casting|CastToMSC_SpellParent (.parent (Variables|Default|GetSpell%20Data))))
  (bind _asmsc_spell_prefab (Utilities|Casting|CastToMSC_SpellPrefab Spell))
  (Default|SpellHit _asmsc_spell_parent (Variables|Default|GetCurrent%20Active%20Spells) _asmsc_spell_prefab))

(event Custom|MSC%20Event%20Tick
  (params (Delta%20Time :type Float%20%28double-precision%29))
  (bind _spell_data (Variables|Default|GetSpell%20Data))
  (bind _current_active_spells (Variables|Default|GetCurrent%20Active%20Spells))
  (|CalculateCooldown Delta%20Time)
  (if (> (Utilities|Array|Length (Variables|Default|GetCurrent%20Active%20Spells)) 0)
    (bind _asmsc_spell_parent (Utilities|Casting|CastToMSC_SpellParent (.parent _spell_data)))
    (Default|SpellEventTickBehaviorBase _asmsc_spell_parent _current_active_spells)
    (for _array_element (.mods _spell_data)
      (bind _asmsc_spell_mod_parent (Utilities|Casting|CastToMSC_SpellModParent _array_element))
      (Default|SpellEventTickBehaviorModification _asmsc_spell_mod_parent _current_active_spells))))

(fn GenerateSpell
  (params (Spell :type Actor%20Component%20Class%20Reference) (Spell%20Mods :type Array%20of%20Actor%20Component%20Class%20References))
  (|CheckValidInput Spell Spell%20Mods)
  (|DestroyOldSpellComponents
    (:Completed
      (|SetSpellData Spell Spell%20Mods)
      (Development|PrintString "Spell Regenerated!" true true "(R=0.000000,G=0.660000,B=1.000000,A=1.000000)" 1e+01))))

(fn IsValidSpell
  (params (TestClass :type Object%20Class%20Reference))
  (return (Utilities|ClassIsChildOf TestClass "/Game/Blueprints/MSC_MagicSystem/MSC_SpellParent.MSC_SpellParent_C")))

(fn IsValidSpellMod
  (params (TestClass :type Object%20Class%20Reference))
  (return (Utilities|ClassIsChildOf TestClass "/Game/Blueprints/MSC_MagicSystem/MSC_SpellModParent.MSC_SpellModParent_C")))