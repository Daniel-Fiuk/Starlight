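; Game Instance that stores global player state: health potions, current spell, spell mods, spell inventory and journal entries.
; Events write the state and getters return it, with spells placed in the inventory by index.
; SetHealthPotions adds to the count and SetCurrentMods appends to the mod list, despite their names.
; Collected journal entries and the notebook's entry list are separate arrays, each with its own add event and getter.
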(event EventSetHealthPotions
  (params (Amount :type Integer))
  (Variables|Default|SetHealthPotions (+ (Variables|Default|GetHealthPotions) Amount)))

(event EventSetCurrentSpell
  (params (SpellInfo :type S%20Spell%20Info%20Structure))
  (Variables|Default|SetCurrentSpell SpellInfo))

(event EventSetCurrentMods
  (params (Mod :type S%20Spell%20Info%20Structure))
  (Utilities|Array|Add (Variables|Default|GetSpellMods) Mod))

(event EventRemoveModatIndex
  (params (Index :type Integer))
  (Utilities|Array|RemoveIndex (Variables|Default|GetSpellMods) Index))

(event EventAddSpelltoInventory
  (params (Spell :type S%20Spell%20Info%20Structure) (Index :type Integer))
  (Utilities|Array|SetArrayElem (Variables|Default|GetSpellInventory) Index Spell))

(event EventAddJournalEntry
  (params (Entry :type Text))
  (Utilities|Array|Add (Variables|Default|GetCollectedJournalEntries) Entry))

(event EventAddJournalEntryList
  (params (Entry :type S%20Journal%20Text%20Structure))
  (Utilities|Array|Add (Variables|Default|GetJournalEntryList) Entry))

(event EventClearMods
  (Utilities|Array|Clear (Variables|Default|GetSpellMods)))

(fn GetCurrentMods
  (return (Variables|Default|GetSpellMods)))

(fn GetCurrentSpell
  (return (Variables|Default|GetCurrentSpell)))

(fn GetHealthPotions
  (return (Variables|Default|GetHealthPotions)))

(fn GetJournalEntriesList
  (return (Variables|Default|GetCollectedJournalEntries)))

(fn GetJournalEntryListNotebook
  (return (Variables|Default|GetJournalEntryList)))

(fn GetSpellInventory
  (return (Variables|Default|GetSpellInventory)))