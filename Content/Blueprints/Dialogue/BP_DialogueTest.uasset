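; Test dialogue actor that lets the main character press E inside its sphere to step through an array of text lines.
; Sphere overlap toggles input and the hotbar's interact prompt, and leaving resets the line index.
; E increments the index before display, so element 0 is skipped, and updates a W_Dialogue widget, removing it after the last line.
; RunDialogue is a print-string variant not called here.
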(event OnComponentBeginOverlap(Sphere)
  (params (OverlappedComponent :type Primitive%20Component%20Object%20Reference) (OtherActor :type Actor%20Object%20Reference) (OtherComp :type Primitive%20Component%20Object%20Reference) (OtherBodyIndex :type Integer) (bFromSweep :type Boolean) (SweepResult :type Hit%20Result%20Structure%20%28by%20ref%29))
  (bind _asbp_main_character (Utilities|Casting|CastToBP_MainCharacter OtherActor))
  (Input|EnableInput (Game|GetPlayerController 0))
  (if (Variables|Default|GetWantText?)
    (Default|ShowInteract (Variables|/Game/Blueprints/BP_MainCharacter.BP_MainCharacter_C|GetHotbarWidgetRef _asbp_main_character))
    (Variables|Default|SetWantText? false)))

(event OnComponentEndOverlap(Sphere)
  (params (OverlappedComponent :type Primitive%20Component%20Object%20Reference) (OtherActor :type Actor%20Object%20Reference) (OtherComp :type Primitive%20Component%20Object%20Reference) (OtherBodyIndex :type Integer))
  (bind _asbp_main_character (Utilities|Casting|CastToBP_MainCharacter OtherActor))
  (Input|DisableInput (Game|GetPlayerController 0) 0)
  (Default|HideInteract (Variables|/Game/Blueprints/BP_MainCharacter.BP_MainCharacter_C|GetHotbarWidgetRef _asbp_main_character))
  (Variables|Default|SetWantText? true)
  (Variables|Default|SetTalkIndex 0))

(event Input|KeyboardEvents|E
  (params (Key :type Key%20Structure :default "None"))
  (:Pressed
    (bind _asbp_main_character (Utilities|Casting|CastToBP_MainCharacter (stale OnComponentBeginOverlap(Sphere) OtherActor)))
    (Default|HideInteract (Variables|/Game/Blueprints/BP_MainCharacter.BP_MainCharacter_C|GetHotbarWidgetRef _asbp_main_character))
    (Variables|Default|SetWantText? false)
    (Math|Integer|IncrementInt (Variables|Default|GetTalkIndex)
      (:%20%20
        (if (< (Variables|Default|GetTalkIndex) (Utilities|Array|Length (Variables|Default|GetDialogue)))
          (Variables|Default|GetUI
            (:then
              _)
            (:else
              (bind _returnvalue (UserInterface|CreateWidget "/Game/Widgets/W_Dialogue.W_Dialogue_C" (Game|GetPlayerController 0)))
              (bind _output_get (Variables|Default|SetUI _returnvalue))
              (UserInterface|Viewport|AddtoViewport _output_get 0)))
          (Rendering|Components|TextRender|SetText (Variables|/Game/Widgets/W_Dialogue.W_Dialogue_C|GetDialogueText (Variables|Default|GetUI)) (Utilities|Text|ToText(String) (Utilities|Array|Get(acopy) (Variables|Default|GetDialogue) (Variables|Default|GetTalkIndex))))
          (else
            (Widget|RemovefromParent (Variables|Default|GetUI))))))))

(fn ConstructionScript)

(fn RunDialogue
  (Math|Integer|IncrementInt (Variables|Default|GetTalkIndex)
    (:%20%20
      (if (<= (Variables|Default|GetTalkIndex) (Utilities|Array|Length (Variables|Default|GetDialogue)))
        (Development|PrintString (Utilities|Array|Get(acopy) (Variables|Default|GetDialogue) (Variables|Default|GetTalkIndex)))))))