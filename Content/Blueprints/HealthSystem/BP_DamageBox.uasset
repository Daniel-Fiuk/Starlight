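; BP_DamageBox is a fire hazard that deals continuous damage to the main character while it stands inside the DamageBox component.
; It spawns a fire particle emitter at its location on BeginPlay.
; Begin overlap caches the BP_MainCharacter and starts a looping timer that applies small, frequent ticks of damage through ApplyDamage.
; End overlap by the character clears that timer to stop the damage.
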(event OnComponentBeginOverlap(DamageBox)
  (params (OverlappedComponent :type Primitive%20Component%20Object%20Reference) (OtherActor :type Actor%20Object%20Reference) (OtherComp :type Primitive%20Component%20Object%20Reference) (OtherBodyIndex :type Integer) (bFromSweep :type Boolean) (SweepResult :type Hit%20Result%20Structure%20%28by%20ref%29))
  (bind _asbp_main_character (Utilities|Casting|CastToBP_MainCharacter OtherActor))
  (Variables|Default|SetAs%20BP%20Main%20Character _asbp_main_character)
  (bind _returnvalue (Utilities|Time|SetTimerbyEvent (delegate Custom|DamagePlayer) 0.1 true))
  (Variables|Default|SetTimerRef _returnvalue))

(event OnComponentEndOverlap(DamageBox)
  (params (OverlappedComponent :type Primitive%20Component%20Object%20Reference) (OtherActor :type Actor%20Object%20Reference) (OtherComp :type Primitive%20Component%20Object%20Reference) (OtherBodyIndex :type Integer))
  (Utilities|Casting|CastToBP_MainCharacter OtherActor)
  (Utilities|Time|ClearandInvalidateTimerbyHandle (Variables|Default|GetTimerRef)))

(event Custom|DamagePlayer
  (Game|Damage|ApplyDamage (Variables|Default|GetAs%20BP%20Main%20Character) 0.5 0 0))

(event EventBeginPlay
  (Effects|SpawnEmitteratLocation "/Game/StarterContent/Particles/P_Fire.P_Fire" (Transformation|GetActorLocation)))

(fn ConstructionScript)