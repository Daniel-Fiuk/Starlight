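; BP_HealthBox is a healing zone that gradually restores BP_MainCharacter's health while the character stands inside its HealBox.
; It spawns a spark particle effect at its location on BeginPlay.
; Entering the box starts a looping timer that adds a small health increment per tick unless health exactly equals the hardcoded maximum.
; Leaving the box clears the timer.
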(event OnComponentBeginOverlap(HealBox)
  (params (OverlappedComponent :type Primitive%20Component%20Object%20Reference) (OtherActor :type Actor%20Object%20Reference) (OtherComp :type Primitive%20Component%20Object%20Reference) (OtherBodyIndex :type Integer) (bFromSweep :type Boolean) (SweepResult :type Hit%20Result%20Structure%20%28by%20ref%29))
  (bind _asbp_main_character (Utilities|Casting|CastToBP_MainCharacter OtherActor))
  (bind _returnvalue (Utilities|Time|SetTimerbyEvent (delegate Custom|HealPlayer) 0.1 true))
  (Variables|Default|SetTimerRef _returnvalue))

(event OnComponentEndOverlap(HealBox)
  (params (OverlappedComponent :type Primitive%20Component%20Object%20Reference) (OtherActor :type Actor%20Object%20Reference) (OtherComp :type Primitive%20Component%20Object%20Reference) (OtherBodyIndex :type Integer))
  (Utilities|Casting|CastToBP_MainCharacter OtherActor)
  (Utilities|Time|ClearandInvalidateTimerbyHandle (Variables|Default|GetTimerRef)))

(event Custom|HealPlayer
  (if (not (== (Variables|/Game/Blueprints/Player/BP_MainCharacter.BP_MainCharacter_C|GetHealth (stale OnComponentBeginOverlap(HealBox) _asbp_main_character)) 1e+02))
    (Variables|/Game/Blueprints/Player/BP_MainCharacter.BP_MainCharacter_C|SetHealth (stale OnComponentBeginOverlap(HealBox) _asbp_main_character) (+ (Variables|/Game/Blueprints/Player/BP_MainCharacter.BP_MainCharacter_C|GetHealth (stale OnComponentBeginOverlap(HealBox) _asbp_main_character)) 0.5))))

(event EventBeginPlay
  (Effects|SpawnEmitteratLocation "/Game/StarterContent/Particles/P_Sparks.P_Sparks" (Transformation|GetActorLocation)))

(fn ConstructionScript)